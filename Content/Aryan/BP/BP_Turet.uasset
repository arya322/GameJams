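; Auto-turret that locks onto one random BP_Enemy inside its detection sphere and shoots BP_Bullet at it.
; Tick smoothly rotates the top and snaps the firing arrow toward the target, reselecting when it is lost.
; A looping timer drives firing, which drains ammo and battery.
; A proximity-shown widget button requests reloads paid from the player's Bullet/Battery inventory, though BeginPlay zeroes MaxBullets, blocking refills.
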(event OnComponentBeginOverlap(Sphere)
  (params (OverlappedComponent :type Primitive%20Component%20Object%20Reference) (OtherActor :type Actor%20Object%20Reference) (OtherComp :type Primitive%20Component%20Object%20Reference) (OtherBodyIndex :type Integer) (bFromSweep :type Boolean) (SweepResult :type Hit%20Result%20Structure%20%28by%20ref%29))
  ;[0.105 0.23 0.31] 01  /  ENEMY DETECTION + TARGET LOCK
  (Utilities|Casting|CastToBP_Enemy OtherActor)
  (CallFunction|T13SelectEnemy))

(event OnComponentBeginOverlap(C_Button)
  (params (OverlappedComponent :type Primitive%20Component%20Object%20Reference) (OtherActor :type Actor%20Object%20Reference) (OtherComp :type Primitive%20Component%20Object%20Reference) (OtherBodyIndex :type Integer) (bFromSweep :type Boolean) (SweepResult :type Hit%20Result%20Structure%20%28by%20ref%29))
  ;[0.105 0.23 0.31] 09  /  PLAYER ENTERS C_BUTTON - VISIBLE + CURSOR TRUE
  (Utilities|Casting|CastToBP_ThirdPersonCharacter OtherActor)
  (Variables|Default|SetbPlayerInButtonRange true)
  (Rendering|SetVisibility (Variables|Default|GetButton) true false)
  (Variables|/Script/Engine.PlayerController|SetbShowMouseCursor (Game|GetPlayerController 0) true))

(event OnComponentEndOverlap(C_Button)
  (params (OverlappedComponent :type Primitive%20Component%20Object%20Reference) (OtherActor :type Actor%20Object%20Reference) (OtherComp :type Primitive%20Component%20Object%20Reference) (OtherBodyIndex :type Integer))
  ;[0.105 0.23 0.31] 10  /  PLAYER LEAVES C_BUTTON - HIDDEN + CURSOR FALSE
  (Utilities|Casting|CastToBP_ThirdPersonCharacter OtherActor)
  (Variables|Default|SetbPlayerInButtonRange false)
  (Rendering|SetVisibility (Variables|Default|GetButton) false false)
  (Variables|/Script/Engine.PlayerController|SetbShowMouseCursor (Game|GetPlayerController 0) false))

(event OnComponentEndOverlap(Sphere)
  (params (OverlappedComponent :type Primitive%20Component%20Object%20Reference) (OtherActor :type Actor%20Object%20Reference) (OtherComp :type Primitive%20Component%20Object%20Reference) (OtherBodyIndex :type Integer))
  ;[0.105 0.23 0.31] 03  /  ENEMY LEAVES RANGE
  (if (== OtherActor (Variables|Default|GetTargetEnemy))
    (Variables|Default|SetTargetEnemy 0)
    (CallFunction|T13SelectEnemy)))

(event Custom|T13_InitializeReloadWidget
  ;[0.105 0.23 0.31] 08  /  INITIALIZE WBP_BUTTON AND SET OWNING TURRET
  (bind _aswbp_button (Utilities|Casting|CastToWBP_Button (UserInterface|GetUserWidgetObject (Variables|Default|GetButton)))
    (:then
      (Variables|/Game/Aryan/UI/WBP_Button.WBP_Button_C|SetTurretRef _aswbp_button self)
      (Rendering|SetVisibility (Variables|Default|GetButton) false false))
    (:CastFailed
      (Development|PrintString "Hello"))))

(event Custom|T13_SelectEnemy
  (bind _sphere (Variables|Default|GetSphere))
  (bind _overlappingactors (Collision|GetOverlappingActors _sphere "/Game/ThirdPerson/Blueprints/BP_Enemy.BP_Enemy_C" :!class /Script/Engine.PrimitiveComponent))
  (bind _returnvalue (Utilities|Array|Length _overlappingactors))
  ;[0.105 0.23 0.31] 01  /  ENEMY DETECTION + TARGET LOCK
  (if (not (Utilities|IsValid (Variables|Default|GetTargetEnemy)))
    (if (> _returnvalue 0)
      (bind _asbp_enemy (Utilities|Casting|CastToBP_Enemy (Utilities|Array|Get(acopy) _overlappingactors (Math|Random|RandomInteger _returnvalue))))
      (Variables|Default|SetTargetEnemy _asbp_enemy)
      (Development|PrintString "LOCKED: ONE ENEMY"))))

(event Custom|T13_PaidReload
  ;[0.105 0.23 0.31] 06  /  PAID RELOAD - PLAYER BULLET + BATTERY INVENTORY
  (if (Variables|Default|GetIsReloading)
    (Development|PrintString "Hello")
    (else
      (bind _asbp_third_person_character (Utilities|Casting|CastToBP_ThirdPersonCharacter (Game|GetPlayerCharacter 0))
        (:then
          (Variables|Default|SetReloadWorkingInventory (Variables|/Game/ThirdPerson/Blueprints/BP_ThirdPersonCharacter.BP_ThirdPersonCharacter_C|GetInventory _asbp_third_person_character))
          (if (> (- (Variables|Default|GetMaxBullets) (Variables|Default|GetCurrentBullets)) 0)
            (if (>= (.Value (Utilities|Map|Find (Variables|Default|GetReloadWorkingInventory) "Bullet")) (- (Variables|Default|GetMaxBullets) (Variables|Default|GetCurrentBullets)))
              (if (>= (.Value (Utilities|Map|Find (Variables|Default|GetReloadWorkingInventory) "Battery")) 0)
                (Utilities|Map|Add (Variables|Default|GetReloadWorkingInventory) "Bullet" (- (.Value (Utilities|Map|Find (Variables|Default|GetReloadWorkingInventory) "Bullet")) (- (Variables|Default|GetMaxBullets) (Variables|Default|GetCurrentBullets))))
                (Utilities|Map|Add (Variables|Default|GetReloadWorkingInventory) "Battery" (- (.Value (Utilities|Map|Find (Variables|Default|GetReloadWorkingInventory) "Battery")) 1))
                (Variables|/Game/ThirdPerson/Blueprints/BP_ThirdPersonCharacter.BP_ThirdPersonCharacter_C|SetInventory _asbp_third_person_character (Variables|Default|GetReloadWorkingInventory))
                (Variables|Default|SetIsReloading false)
                (Utilities|FlowControl|Delay (Variables|Default|GetReloadDuration))
                (Variables|Default|SetCurrentBullets (Variables|Default|GetMaxBullets))
                (Variables|Default|SetCurrentBattery (Variables|Default|GetMaxBattery))
                (Variables|Default|SetIsReloading false)
                (Development|PrintString "Hello")
                (else
                  (Development|PrintString "Hello")))
              (else
                (Development|PrintString "Hello")))
            (else
              (Development|PrintString "Hello"))))
        (:CastFailed
          (Development|PrintString "Hello"))))))

(event Custom|RequestReloadFromButton
  ;[0.105 0.23 0.31] 11  /  WBP_BUTTON ONCLICKED -> REQUEST PAID RELOAD
  (if (Variables|Default|GetbPlayerInButtonRange)
    (CallFunction|T13PaidReload)
    (else
      (Development|PrintString "Hello"))))

(event Custom|TurretShoot_V6
  (bind _batterydrainpersecond (Variables|Default|GetBatteryDrainPerSecond))
  (bind _shootinterval (Variables|Default|GetShootInterval))
  (bind _targetenemy (Variables|Default|GetTargetEnemy))
  (bind _returnvalue (* _batterydrainpersecond _shootinterval))
  ;[0.105 0.23 0.31] 05  /  FIRING - BP_BULLET + BATTERY DRAIN
  (if (Utilities|IsValid _targetenemy)
    (if (Collision|IsOverlappingActor (Variables|Default|GetSphere) _targetenemy :!class /Script/Engine.PrimitiveComponent)
      (if (not (Variables|Default|GetIsReloading))
        (if (> (Variables|Default|GetCurrentBullets) 0)
          (if (>= (Variables|Default|GetCurrentBattery) (+ (Variables|Default|GetMinBatteryToOperate) _returnvalue))
            (bind _returnvalue_2 (Game|SpawnActorfromClass "/Game/Aryan/BP/BP_Bullet.BP_Bullet_C" (Transformation|GetWorldTransform (Variables|Default|GetArrow)) "AlwaysSpawn" "SelectDefaultAtRuntime" self 0))
            (if (Utilities|IsValid _returnvalue_2)
              (Variables|Default|SetCurrentBullets (- (Variables|Default|GetCurrentBullets) 1))
              (Variables|Default|SetCurrentBattery (Math|Float|Clamp(Float) (- (Variables|Default|GetCurrentBattery) _returnvalue) 0.0 (Variables|Default|GetMaxBattery)))
              (Development|PrintString "BP_Bullet spawned - bullet and battery consumed" false))))))))

(event Custom|T13_InitTurretStatus
  (bind _aswbp_turret_status (Utilities|Casting|CastToWBP_TurretStatus (UserInterface|GetUserWidgetObject (Variables|Default|GetTurretStatus))))
  (Variables|/Game/Aryan/BP/WBP_TurretStatus.WBP_TurretStatus_C|SetTurretRef _aswbp_turret_status self))

(event EventBeginPlay
  ;[0.105 0.23 0.31] 04  /  BEGIN PLAY - 10 AMMO - TIMER - BOTH WIDGETS
  (Variables|Default|SetMaxBullets 0)
  (Variables|Default|SetCurrentBullets 10)
  (Variables|Default|SetCurrentBattery (Variables|Default|GetMaxBattery))
  (Variables|Default|SetIsReloading false)
  (Variables|Default|SetRotationSpeed 5.0)
  (Utilities|Time|SetTimerbyEvent (EventDispatchers|CreateEvent :!event Custom|TurretShoot_V6) (Variables|Default|GetShootInterval) true)
  (CallFunction|T13InitTurretStatus)
  (CallFunction|T13InitializeReloadWidget))

(event EventTick
  (params (DeltaSeconds :type Float%20%28single-precision%29))
  (bind _arrow (Variables|Default|GetArrow))
  (bind _targetenemy (Variables|Default|GetTargetEnemy))
  (bind _top (Variables|Default|GetTop))
  (bind _returnvalue (Transformation|GetActorLocation _targetenemy))
  ;[0.105 0.23 0.31] 02  /  TRACKING + TURRET ROTATION
  (if (Utilities|IsValid _targetenemy)
    (Transformation|SetWorldRotation _top (Math|Interpolation|RInterpTo (Transformation|GetWorldRotation _top) (Math|Rotator|FindLookatRotation (Transformation|GetWorldLocation _top) _returnvalue) DeltaSeconds (Variables|Default|GetRotationSpeed)) false false)
    (Transformation|SetWorldRotation _arrow (Math|Rotator|FindLookatRotation (Transformation|GetWorldLocation _arrow) _returnvalue) false false)
    (else
      (CallFunction|T13SelectEnemy))))

(fn ConstructionScript)

(fn ReloadBullets)