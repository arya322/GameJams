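; BP_DayNight runs a looping day-night cycle that spawns enemies at night.
; A Timeline rotates the Sun between day and night rotations, flipping IsNight at each end and holding briefly before playing the other way.
; While IsNight is set, SpawnEnemy re-calls itself every SpawnInterval, spawning a BP_AI at a random navigable point around the actor.
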(event Custom|SpawnEnemy
  (if (Variables|Default|GetIsNight)
    (bind _randomlocation (Class|NavigationSystemV1|GetRandomLocationinNavigableRadius (Transformation|GetActorLocation) 0.0 0 "/Script/AIModule.NavFilter_AIControllerDefault"))
    (Game|SpawnActorfromClass "/Game/Keira/BP_AI.BP_AI_C" (Math|Transform|MakeTransform _randomlocation) "AdjustIfPossibleButAlwaysSpawn" "MultiplyWithRoot" 0 0)
    (Utilities|FlowControl|Delay (Variables|Default|GetSpawnInterval))
    (CallFunction|SpawnEnemy)))

(event EventBeginPlay
  (Transformation|SetWorldRotation (Variables|Default|GetSun) (Variables|Default|GetDayRotation) false false)
  (Utilities|FlowControl|Delay 1.0)
  (bind _alpha (Timeline|Timeline PlayFromStart)
    (:Update
      (Transformation|SetWorldRotation (Variables|Default|GetSun) (Math|Rotator|Lerp(Rotator) (Variables|Default|GetDayRotation) (Variables|Default|GetNightRotation) _alpha) false false))
    (:Finished
      (if (Variables|Default|GetIsNight)
        (Variables|Default|SetIsNight false)
        (Utilities|FlowControl|Delay 1e+01)
        (Timeline|Timeline PlayFromStart)
        (else
          (Variables|Default|SetIsNight true)
          (CallFunction|SpawnEnemy)
          (Utilities|FlowControl|Delay 1e+01)
          (Timeline|Timeline ReverseFromEnd))))))

(fn ConstructionScript)