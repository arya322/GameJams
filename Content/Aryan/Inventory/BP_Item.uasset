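; BP_Item is a world pickup that adds its ItemID and Quantity to the player's inventory on overlap.
; The PickupBox overlap accepts only an uncollected item with positive quantity touched by BP_ThirdPersonCharacter, then flags it collected.
; It copies the character's Inventory map, adds Quantity to any existing count and writes the map back.
; The actor destroys itself only if the character's HUDRef is valid, though no HUD update occurs here.
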(event OnComponentBeginOverlap(PickupBox)
  (params (OverlappedComponent :type Primitive%20Component%20Object%20Reference) (OtherActor :type Actor%20Object%20Reference) (OtherComp :type Primitive%20Component%20Object%20Reference) (OtherBodyIndex :type Integer) (bFromSweep :type Boolean) (SweepResult :type Hit%20Result%20Structure%20%28by%20ref%29))
  (bind _itemid (Variables|Default|GetItemID))
  ;[1 1 1] 01 | PICKUP OVERLAP: ONLY PLAYER + VALID QUANTITY
  (if (not (Variables|Default|GetHasBeenCollected))
    (if (> (Variables|Default|GetQuantity) 0)
      (bind _asbp_third_person_character (Utilities|Casting|CastToBP_ThirdPersonCharacter OtherActor))
      ;[1 1 1] 02 | COPY PLAYER INVENTORY MAP BEFORE MODIFYING
      (Variables|Default|SetHasBeenCollected true)
      (Variables|Default|SetWorkingInventory (Variables|/Game/ThirdPerson/Blueprints/BP_ThirdPersonCharacter.BP_ThirdPersonCharacter_C|GetInventory _asbp_third_person_character))
      ;[1 1 1] 04 | SAVE UPDATED MAP TO PLAYER; ONLY THEN DESTROY PICKUP
      (Utilities|Map|Add (Variables|Default|GetWorkingInventory) _itemid (+ (.Value (Utilities|Map|Find (Variables|Default|GetWorkingInventory) _itemid)) (Variables|Default|GetQuantity)))
      (Variables|/Game/ThirdPerson/Blueprints/BP_ThirdPersonCharacter.BP_ThirdPersonCharacter_C|SetInventory _asbp_third_person_character (Variables|Default|GetWorkingInventory))
      (Development|PrintString "PICKUP SAVED TO PLAYER INVENTORY")
      (if (Utilities|IsValid (Variables|/Game/ThirdPerson/Blueprints/BP_ThirdPersonCharacter.BP_ThirdPersonCharacter_C|GetHUDRef _asbp_third_person_character))
        (Actor|DestroyActor)))))

(fn ConstructionScript)